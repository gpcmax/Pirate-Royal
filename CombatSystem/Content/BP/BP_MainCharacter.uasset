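; Main player character Blueprint with a sword and gun, plus a pause menu.
; The construction script snaps weapon meshes to hand, sheath or back sockets based on the Sword and Gun flags.
; P or gamepad Special Right creates the UI_Pause widget.
; An unconnected sword hit check line-traces blade points from saved to current positions and calls Hit, which clears CanSwing; BeginPlay and Tick are empty.
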(event EventBeginPlay)

(event EventTick
  (params (DeltaSeconds :type Float%20%28single-precision%29))
  ;[1 1 1] Tick
)

(event Input|KeyboardEvents|P
  (params (Key :type Key%20Structure))
  (:Pressed
    (bind _playerindex (Class|TurnBasedBlueprintLibrary|GetMyPlayerIndex))
    (bind _returnvalue (UserInterface|CreateWidget "/Game/UI/UI_Pause.UI_Pause_C" (Game|GetPlayerController _playerindex)))
    (UserInterface|Viewport|AddtoViewport _returnvalue 0)))

(event Input|GamepadEvents|GamepadSpecialRight
  (params (Key :type Key%20Structure))
  (:Pressed
    (bind _playerindex (Class|TurnBasedBlueprintLibrary|GetMyPlayerIndex))
    (bind _returnvalue (UserInterface|CreateWidget "/Game/UI/UI_Pause.UI_Pause_C" (Game|GetPlayerController _playerindex)))
    (UserInterface|Viewport|AddtoViewport _returnvalue 0)))

(fn ConstructionScript
  (bind _mesh (Variables|Character|GetMesh))
  (bind _mesh_2 (Variables|Character|GetMesh))
  (if (Variables|Default|Getsword)
    (Transformation|AttachComponentToComponent (Variables|Default|GetSM_Sheath) _mesh "Sheath" "SnapToTarget" "SnapToTarget" "SnapToTarget" true)
    (Transformation|AttachComponentToComponent (Variables|Default|GetSM_Sword) _mesh "Sword_Hand" "SnapToTarget" "SnapToTarget" "SnapToTarget" true)
    (elif (Variables|Default|GetGun)
      (Transformation|AttachComponentToComponent (Variables|Default|GetSM_Gun) _mesh_2 "Gun_Hand" "SnapToTarget" "SnapToTarget" "SnapToTarget" true)
      (else
        (Transformation|AttachComponentToComponent (Variables|Default|GetSM_Sheath) _mesh_2 "Sheath" "SnapToTarget" "SnapToTarget" "SnapToTarget" true)
        (Transformation|AttachComponentToComponent (Variables|Default|GetSM_Sword) _mesh_2 "SwordInSheath" "SnapToTarget" "SnapToTarget" "SnapToTarget" true)
        (Transformation|AttachComponentToComponent (Variables|Default|GetSM_Gun) _mesh_2 "RifleOnBack" "SnapToTarget" "SnapToTarget" "SnapToTarget" true)))))

(fn Hit
  (params (Hit :type Hit%20Result%20Structure))
  (Variables|Default|SetbCanSwing false))