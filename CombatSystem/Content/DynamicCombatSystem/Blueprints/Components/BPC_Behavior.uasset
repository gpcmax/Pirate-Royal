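; BPC_Behavior is an actor component in the Dynamic Combat System that classifies other actors as enemies or dangers.
; IsEnemy and IsDanger pass the given actor and the component's Enemies or Danger class array to CheckClass.
; CheckClass returns true when the actor's class is a child of any listed class, so subclasses of a listed class also match.
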(event EventBeginPlay)

(event EventTick
  (params (DeltaSeconds :type Float%20%28single-precision%29)))

(fn IsEnemy
  (params (Actor :type Actor%20Object%20Reference))
  (return (CallFunction|CheckClass Actor (Variables|Default|GetEnemies))))

(fn CheckClass
  (params (Actor :type Actor%20Object%20Reference) (Array :type Array%20of%20Actor%20Class%20References))
  (for _array_element Array
    (if (Utilities|ClassIsChildOf (Utilities|GetClass Actor) _array_element)
      (return true)))
  (return false))

(fn IsDanger
  (params (Actor :type Actor%20Object%20Reference))
  (return (CallFunction|CheckClass Actor (Variables|Default|GetDanger))))